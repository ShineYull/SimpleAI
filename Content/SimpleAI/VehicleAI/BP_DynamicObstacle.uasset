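; Moving obstacle actor for the simple vehicle AI that shuttles back and forth along its right vector around its start position.
; On BeginPlay it stores that position, passes its BoxCollision to the ACMotionTrajectory component and spawns a force field from it.
; Unless paused, Tick steps it by Speed, flipping direction past MovementRange on either side; the step is not scaled by delta time.
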(event EventBeginPlay
  (Variables|Default|SetActorLocation (Transformation|GetActorLocation))
  (Variables|/Game/SimpleAI/VehicleAI/AC_MotionTrajectory.AC_MotionTrajectory_C|SetBoxCollision (Variables|Default|GetAC_MotionTrajectory) (Variables|Default|GetBoxCollision))
  (Default|SpawnForceField (Variables|Default|GetAC_MotionTrajectory)))

(event Collision|EventActorBeginOverlap
  (params (OtherActor :type Actor%20Object%20Reference)))

(event EventTick
  (params (DeltaSeconds :type Float%20%28single-precision%29))
  (if (not (Variables|Default|GetbIsPause))
    (Utilities|FlowControl|Sequence
      (:then_0
        (if (> (Math|Vector|DotProduct (- (Transformation|GetActorLocation) (Variables|Default|GetActorLocation)) (Transformation|GetActorRightVector)) (Variables|Default|GetMovementRange))
          (Variables|Default|SetbIsAddOrSubtract false)))
      (:then_1
        (if (< (Math|Vector|DotProduct (- (Transformation|GetActorLocation) (Variables|Default|GetActorLocation)) (Transformation|GetActorRightVector)) (* (Variables|Default|GetMovementRange) -1.0))
          (Variables|Default|SetbIsAddOrSubtract true)))
      (:then_2
        (if (Variables|Default|GetbIsAddOrSubtract)
          (Transformation|SetActorRelativeLocation (+ (Transformation|GetActorLocation) (* (Transformation|GetActorRightVector) (Variables|Default|GetSpeed))))
          (else
            (Transformation|SetActorRelativeLocation (+ (Transformation|GetActorLocation) (* (Transformation|GetActorRightVector) (* (Variables|Default|GetSpeed) -1.0))))))))))

(fn ConstructionScript)