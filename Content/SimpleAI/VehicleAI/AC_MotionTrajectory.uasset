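; Vehicle AI component that predicts its owner's motion trajectory and can line the predicted path with force field actors.
; A looping timer records a capped position history, feeds it to PredictFuturePositions with a Degree setting, and flattens results to owner height.
; SpawnForceField creates box-sized BP_ForceField actors, which each update moves onto predicted points.
; Their path-aligned yaw branch requires a negative index, so they always take the owner's yaw.
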(event Custom|UpdateHistoryPositionsEvent
  (CallFunction|TrackActorPositions)
  (bind _returnvalue (Class|AlgorithmBPLibrary|PredictFuturePositions (Variables|Default|GetHistoryPositions) (Variables|Default|GetDegree) (Variables|Default|GetMaxFuturePosition) 1.0))
  (Variables|Default|SetFuturePositions _returnvalue)
  (for (_array_element _array_index) (Variables|Default|GetFuturePositions)
    (Utilities|Array|SetArrayElem (Variables|Default|GetFuturePositions) _array_index (Math|Vector|MakeVector (.X (Math|Vector|BreakVector _array_element)) (.Y (Math|Vector|BreakVector _array_element)) (.z (Transformation|GetActorLocation (Components|GetOwner)))))
    (if (Variables|Debug|GetbIsDebugPath)
      (Rendering|Debug|DrawDebugSphere (Math|Vector|MakeVector (.X (Math|Vector|BreakVector _array_element)) (.Y (Math|Vector|BreakVector _array_element)) (.z (Transformation|GetActorLocation (Components|GetOwner)))) 3e+01 12 "(R=0.000000,G=1.000000,B=0.000000,A=1.000000)" 0.0 2.0)))
  (if (Variables|Default|GetbIsForceField)
    (CallFunction|UpdateForceField)))

(event Custom|SpawnForceField
  (Utilities|IsValid (Variables|Default|GetBoxCollision)
    (:Is%20Valid
      (for _index (range 0 (- (Variables|Default|GetMaxFuturePosition) 1))
        (bind _returnvalue (Game|SpawnActorfromClass "/Game/SimpleAI/VehicleAI/BP_ForceField.BP_ForceField_C" (Math|Transform|MakeTransform "0, 0, 0" "0, 0, 0" "1.000000,1.000000,1.000000") "Undefined" "MultiplyWithRoot" (Components|GetOwner) 0))
        (Utilities|Array|Add (Variables|Default|GetForceFields) _returnvalue)
        (Components|Box|SetBoxExtent (Variables|/Game/SimpleAI/VehicleAI/BP_ForceField.BP_ForceField_C|GetBoxCollision _returnvalue) (Variables|/Script/Engine.BoxComponent|GetBoxExtent (Variables|Default|GetBoxCollision)) true)
        (if (Variables|Debug|GetbIsDebugForceField)
          (Development|SetHiddeninGame (Variables|/Game/SimpleAI/VehicleAI/BP_ForceField.BP_ForceField_C|GetBoxCollision _returnvalue) false false)
          (else
            (Development|SetHiddeninGame (Variables|/Game/SimpleAI/VehicleAI/BP_ForceField.BP_ForceField_C|GetBoxCollision _returnvalue) true false))))
      (Variables|Default|SetbIsForceField true))))

(event EventBeginPlay
  (Utilities|Time|SetTimerbyFunctionName 0 "UpdateHistoryPositionsEvent" (Variables|Default|GetUpdateTime) true))

(event EventTick
  (params (DeltaSeconds :type Float%20%28single-precision%29)))

(fn TrackActorPositions
  (Utilities|FlowControl|Sequence
    (:then_0
      (Utilities|IsValid (Components|GetOwner)
        (:Is%20Valid
          (LocalVariables|SetLocal_CurrentPosition (Transformation|GetActorLocation (Components|GetOwner)))
          (Utilities|Array|Add (Variables|Default|GetHistoryPositions) (LocalVariables|GetLocal_CurrentPosition))
          (LocalVariables|SetLocal_Complete (> (Utilities|Array|Length (Variables|Default|GetHistoryPositions)) (Variables|Default|GetMaxHistoryPosition)))
          (if (LocalVariables|GetLocal_Complete)
            (Utilities|Array|RemoveIndex (Variables|Default|GetHistoryPositions))))))
    (:then_1
      (if (Variables|Debug|GetbIsDebugPath)
        (Rendering|Debug|DrawDebugSphere (LocalVariables|GetLocal_CurrentPosition) 3e+01 12 "(R=1.000000,G=0.000000,B=0.000000,A=1.000000)" (* (Variables|Default|GetUpdateTime) (Variables|Default|GetMaxHistoryPosition)) 2.0)))
    (:then_2
      (return (LocalVariables|GetLocal_Complete)))))

(fn UpdateForceField
  (Utilities|IsValid (Variables|Default|GetBoxCollision)
    (:Is%20Valid
      (for (_array_element _array_index) (Variables|Default|GetFuturePositions)
        (LocalVariables|SetLocal_ArrayIndex _array_index)
        (if (and (< _array_index 0) (>= (Math|Vector|Distance(Vector) (Utilities|Array|Get(acopy) (Variables|Default|GetFuturePositions) _array_index) (Transformation|GetActorLocation (Components|GetOwner))) 2e+02))
          (Transformation|SetActorLocationAndRotation (Utilities|Array|Get(acopy) (Variables|Default|GetForceFields) (LocalVariables|GetLocal_ArrayIndex)) (Math|Vector|MakeVector (.X (Math|Vector|BreakVector _array_element)) (.Y (Math|Vector|BreakVector _array_element)) (.z (Transformation|GetWorldLocation (Variables|Default|GetBoxCollision)))) (Math|Rotator|MakeRotator 0.0 0.0 (.Yaw (Math|Rotator|BreakRotator (Math|Rotator|CombineRotators (Math|Conversions|RotationFromXVector (Math|Vector|GetUnitDirection(Vector) (Utilities|Array|Get(acopy) (Variables|Default|GetFuturePositions) (- _array_index 1)) (Utilities|Array|Get(acopy) (Variables|Default|GetFuturePositions) _array_index))) (Math|Rotator|Delta(Rotator) (Math|Conversions|RotationFromXVector (Math|Vector|GetUnitDirection(Vector) (Utilities|Array|Get(acopy) (Variables|Default|GetFuturePositions) (- _array_index 1)) (Utilities|Array|Get(acopy) (Variables|Default|GetFuturePositions) _array_index))) (Transformation|GetWorldRotation (Variables|Default|GetBoxCollision))))))))
          (else
            (Transformation|SetActorLocationAndRotation (Utilities|Array|Get(acopy) (Variables|Default|GetForceFields) (LocalVariables|GetLocal_ArrayIndex)) (Math|Vector|MakeVector (.X (Math|Vector|BreakVector _array_element)) (.Y (Math|Vector|BreakVector _array_element)) (.z (Transformation|GetWorldLocation (Variables|Default|GetBoxCollision)))) (Math|Rotator|MakeRotator 0.0 0.0 (.Yaw (Math|Rotator|BreakRotator (Transformation|GetActorRotation (Components|GetOwner))))))))))))