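; BP_Base_AOE is a base area-of-effect actor that detects Pawns within a sphere around its location.
; Trigger runs the check, either when called or automatically after a short BeginPlay delay if TriggerOnBeginPlay is set.
; A one-shot sphere overlap, optionally ignoring the instigator and drawn for debugging, passes each hit actor to the OnAOEOverlapActor dispatcher.
; The effect on those actors is left to whatever binds that dispatcher.
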(event Custom|SpawnAOESphere
  ;[0.15 0.15 0.15 0.5] 生成AOE球体
  (Utilities|FlowControl|Sequence
    (:then_0
      (if (Variables|Default|GetbIsDrawDebugSphere)
        (Rendering|Debug|DrawDebugSphere (Transformation|GetActorLocation) (Variables|Default|GetSphereRadius) 12 "(R=1.000000,G=0.000000,B=0.000000,A=1.000000)" 2.0 1.0)))
    (:then_1
      (bind _outactors (Collision|SphereOverlapActors (Transformation|GetActorLocation) (Variables|Default|GetSphereRadius) (Utilities|Array|MakeArray "ObjectTypeQuery3") 0 (select (Variables|Default|GetbIgnoreInstigator) (Utilities|Array|MakeArray (Game|GetInstigator)) 0)))
      (for _array_element _outactors
        (Default|CallDispatcheronAOEOverlapActor _array_element)))))

(event Custom|Trigger
  (CallFunction|SpawnAOESphere))

(event EventBeginPlay
  (if (Variables|Default|GetbTriggerOnBeginPlay)
    (Utilities|FlowControl|Delay 0.2)
    (CallFunction|Trigger)))

(fn ConstructionScript)