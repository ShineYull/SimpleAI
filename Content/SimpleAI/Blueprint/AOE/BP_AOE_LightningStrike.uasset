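; Lightning strike area-of-effect actor that marks a spot on the floor, then strikes after a delay.
; On BeginPlay it line traces downward from the attack target, ignoring that target, and moves itself to the hit point.
; It spawns a warning decal there, waits, calls Trigger (not defined in this graph) and removes the decal.
; The trace end multiplies the target's Z by -1000 rather than subtracting an offset.
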(event Custom|MoveToFloor
  (Variables|Default|GetAttackTarget
    (:then
      (bind (_outhit _returnvalue) (Collision|LineTraceByChannel (Transformation|GetActorLocation (Variables|Default|GetAttackTarget)) (* (Transformation|GetActorLocation (Variables|Default|GetAttackTarget)) "1.000000,1.000000,-1000.000000") "TraceTypeQuery1" false (Utilities|Array|MakeArray (Variables|Default|GetAttackTarget)) "None"))
      (if _returnvalue
        (Transformation|SetActorLocation (.Location (Collision|BreakHitResult _outhit)) false false)))
    (:else)))

(event EventBeginPlay
  (|CallParentFunction)
  (CallFunction|MovetoFloor)
  (bind _returnvalue (Rendering|Decal|SpawnDecalatLocation (Variables|Default|GetCustomDecalMaterial) "25.000000,256.000000,256.000000" (Transformation|GetActorLocation) "-90.000000,0.000000,0.000000" 0.0))
  (Variables|Default|SetDecal _returnvalue)
  (Utilities|FlowControl|Delay (Variables|Default|GetDelayBeforeStrike))
  (CallFunction|Trigger)
  (Utilities|IsValid (Variables|Default|GetDecal)
    (:Is%20Valid
      (Components|DestroyComponent (Variables|Default|GetDecal)))))

(event Collision|EventActorBeginOverlap
  (params (OtherActor :type Actor%20Object%20Reference))
  (|CallParentFunction OtherActor) ; This node is disabled and will not be called.\nDrag off pins to build functionality.
)

(event EventTick
  (params (DeltaSeconds :type Float%20%28single-precision%29))
  (|CallParentFunction DeltaSeconds) ; This node is disabled and will not be called.\nDrag off pins to build functionality.
)

(fn ConstructionScript
  (|CallParentFunction))