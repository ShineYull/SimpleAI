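; BP_PatrolRoute is a patrol route for enemy AI, defined by the points of a PatrolRoute spline.
; It tracks a current point index and direction, and GetSplinePointAsWorldLocation returns that point's world location.
; IncrementPatrolRoute steps the index and flips direction at the first and last points, so the route runs back and forth instead of looping.
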(event Custom|IncrementPatrolRoute
  (Variables|Default|SetCurrentPatrolIndex (+ (Variables|Default|GetCurrentPatrolIndex) (Variables|Default|GetCurrentDirection)))
  (if (== (Variables|Default|GetCurrentPatrolIndex) (- (Spline|GetNumberOfSplinePoints (Variables|Default|GetPatrolRoute)) 1))
    (Variables|Default|SetCurrentDirection -1)
    (elif (== (Variables|Default|GetCurrentPatrolIndex) 0)
      (Variables|Default|SetCurrentDirection 1))))

(fn ConstructionScript)

(fn GetSplinePointasWorldLocation
  (return (Spline|GetLocationatSplinePoint (Variables|Default|GetPatrolRoute) (Variables|Default|GetCurrentPatrolIndex) "World")))