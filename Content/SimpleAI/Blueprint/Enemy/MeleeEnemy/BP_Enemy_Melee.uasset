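; Sword-wielding melee enemy that supplies the attack, weapon and block actions for an AI character.
; Four attack events pass montage and damage info to BPCAttack for ground smash, slash, jump and spin attacks.
; Draw and sheath montage notifies spawn or destroy the socketed sword, with dispatchers signalling completion.
; TakeDamage randomly starts a timed block for blockable hits before forwarding to BPCDamage, whose blocked callback plays a reaction then ends the block.
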(event DispatcheronBlocked(BPC_Damage)
  (params (InCanBeParried :type Boolean))
  ;[0.15 0.15 0.15 0.5] 格挡招式
  (Variables|Default|SetBlockingState "NewEnumerator2")
  (Utilities|Time|ClearandInvalidateTimerbyHandle (Variables|Default|GetHoldBlockTimer))
  (Animation|Montage|PlayMontage (Variables|Character|GetMesh) "/Game/Characters/Mannequins/Anims/Sword/Block/AM_Sword_Blocking_React.AM_Sword_Blocking_React"
    (:OnCompleted
      _)
    (:OnInterrupted
      _))
  (CallFunction|EndBlock))

(event Custom|StartBlock
  ;[0.15 0.15 0.15 0.5] 格挡招式
  (Utilities|Time|ClearandInvalidateTimerbyHandle (Variables|Default|GetHoldBlockTimer))
  (Components|Movement|StopMovementImmediately (Variables|Character|GetCharacterMovement))
  (Variables|/Game/SimpleAI/Blueprint/Damage_Component/BPC_Damage.BPC_Damage_C|SetbIsBlocking (Variables|Default|GetBPC_Damage) true)
  (Variables|Default|SetBlockingState "NewEnumerator1")
  (bind _returnvalue (Utilities|Time|SetTimerbyEvent (EventDispatchers|CreateEvent :!event Custom|EndBlock) 2.0))
  (Variables|Default|SetHoldBlockTimer _returnvalue))

(event Custom|EndBlock
  ;[0.15 0.15 0.15 0.5] 格挡招式
  (Variables|/Game/SimpleAI/Blueprint/Damage_Component/BPC_Damage.BPC_Damage_C|SetbIsBlocking (Variables|Default|GetBPC_Damage) false)
  (Variables|Default|SetBlockingState "NewEnumerator0")
  (Default|CallDispatcherBlockEnded))

(event Custom|ShortRangeAttack
  (params (InAttackTarget :type Actor%20Object%20Reference))
  ;[0.15 0.15 0.15 0.5] 攻击
  (Default|PrimaryMeleeAttack (Variables|Default|GetBPC_Attack) (Utilities|Struct|MakeS_AttackInfo InAttackTarget "/Game/Characters/Mannequins/Anims/Sword/Attack/AM_Sword_Slash.AM_Sword_Slash" (Utilities|Struct|MakeS_DamageInfo 1e+01 "NewEnumerator1")) 2e+01 2e+02))

(event Custom|LongRangeAttack
  (params (InAttackTarget :type Actor%20Object%20Reference))
  ;[0.15 0.15 0.15 0.5] 攻击
  (Default|LongRangeMeleeAttack (Variables|Default|GetBPC_Attack) (Utilities|Struct|MakeS_AttackInfo InAttackTarget "/Game/Characters/Mannequins/Anims/Sword/Attack/AM_Sword_Jump_Attack.AM_Sword_Jump_Attack" (Utilities|Struct|MakeS_DamageInfo 1e+01 "NewEnumerator1")) 2e+01 2e+02))

(event Custom|GroundSmashAttack
  (params (InAttackTarget :type Actor%20Object%20Reference))
  ;[0.15 0.15 0.15 0.5] 攻击
  (Default|GroundSmash (Variables|Default|GetBPC_Attack) (Utilities|Struct|MakeS_AttackInfo InAttackTarget "/Game/Characters/Mannequins/Anims/Sword/Attack/AM_Sword_Ground_Smash.AM_Sword_Ground_Smash" (Utilities|Struct|MakeS_DamageInfo 25.0 "NewEnumerator3")) 3e+02))

(event Custom|SpinningAttack
  (params (InAttackTarget :type Actor%20Object%20Reference))
  ;[0.15 0.15 0.15 0.5] 攻击
  (Default|SpinningAttack (Variables|Default|GetBPC_Attack) (Utilities|Struct|MakeS_AttackInfo InAttackTarget "/Game/Characters/Mannequins/Anims/Sword/Attack/AM_Sword_Spinning_Attack.AM_Sword_Spinning_Attack" (Utilities|Struct|MakeS_DamageInfo 1e+01 "NewEnumerator1")) 2e+02))

(event EventUnequipWeapon
  ;[0.15 0.15 0.15 0.5] 收剑
  (bind _notifyname (Animation|Montage|PlayMontage (Variables|Character|GetMesh) "/Game/Characters/Mannequins/Anims/Sword/DrawAndSheathSword/AM_Sheath_Sword.AM_Sheath_Sword")
    (:OnCompleted
      (Default|CallDispatcherUnequipWeaponCompleted))
    (:OnNotifyBegin
      (switch name _notifyname
        (:DropSword
          (Actor|DestroyActor (Variables|Default|GetWeaponActor))
          (Variables|Default|SetbIsWieldingWeapon false))))))

(event EventEquipWeapon
  ;[0.15 0.15 0.15 0.5] 拔剑
  (bind _notifyname (Animation|Montage|PlayMontage (Variables|Character|GetMesh) "/Game/Characters/Mannequins/Anims/Sword/DrawAndSheathSword/AM_Draw_Sword.AM_Draw_Sword")
    (:OnCompleted
      (Default|CallDispatcherEquipWeaponCompleted))
    (:OnNotifyBegin
      (switch name _notifyname
        (:HoldSword
          (bind _returnvalue (Game|SpawnActorfromClass "/Game/SimpleAI/Blueprint/Weapon/BP_Weapon_Sword.BP_Weapon_Sword_C" (Transformation|GetActorTransform) "Undefined" "MultiplyWithRoot" 0 0))
          (Variables|Default|SetWeaponActor _returnvalue)
          (Transformation|AttachComponentToComponent (Variables|Default|GetWeaponActor) (Variables|Character|GetMesh) "Hand_R_Sword_Socket" "SnapToTarget" "SnapToTarget" "SnapToTarget" true)
          (Variables|Default|SetbIsWieldingWeapon true))))))

(event EventBeginPlay
  ;[0.15 0.15 0.15 0.5] 初始化
  (|CallParentFunction))

(fn ConstructionScript
  (|CallParentFunction)
  (Variables|Event_SpinMesh|SetMeshRotationBeforeSpin (Variables|/Script/Engine.SceneComponent|GetRelativeRotation (Variables|Character|GetMesh))))

(fn TakeDamage
  (params (InDamageInfo :type S%20Damage%20Info%20Structure) (DamageCauser :type Actor%20Object%20Reference))
  (Utilities|FlowControl|Sequence
    (:then_0
      (if (Utilities|Struct|BreakS_DamageInfo InDamageInfo)
        (CallFunction|TrytoBlock)))
    (:then_1
      (bind _outwasdamaged (Default|TakeDamage (Variables|Default|GetBPC_Damage) InDamageInfo DamageCauser))
      (return _outwasdamaged))))

(fn TrytoBlock
  (if (<= (Math|Random|RandomFloat) (Variables|Default|GetBlockChance))
    (CallFunction|StartBlock)))

(fn GetIdealRange
  (return 2e+02 4e+02))

(fn CalculateFutureActorLocation
  (params (InActor :type Actor%20Object%20Reference) (InTime :type Float%20%28double-precision%29))
  (return (+ (Transformation|GetActorLocation InActor) (* (* (Transformation|GetVelocity InActor) "1.000000,1.000000,0.000000") InTime))))