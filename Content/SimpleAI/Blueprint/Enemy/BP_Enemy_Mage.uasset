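; Mage enemy Blueprint for the SimpleAI system that attacks its target with a fireball spell.
; Attack calls the parent, then plays a fireball montage whose notify triggers BPCAttack to cast a magic spell from the right hand at the target with fixed damage.
; Montage completion or interruption both end the attack.
; It also maps speed types to walk speeds and supplies ideal attack and defend ranges.
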(event EventBeginPlay
  (|CallParentFunction) ; This node is disabled and will not be called.\nDrag off pins to build functionality.
)

(event Collision|EventActorBeginOverlap
  (params (OtherActor :type Actor%20Object%20Reference)))

(event EventTick
  (params (DeltaSeconds :type Float%20%28single-precision%29)))

(event EventAttack
  (params (InAttackTarget :type Actor%20Object%20Reference))
  (bind _output_get (Variables|Event_Attack|SetAttack_InAttackTarget InAttackTarget))
  (|CallParentFunction _output_get)
  (bind _notifyname (Animation|Montage|PlayMontage (Variables|Character|GetMesh) "/Game/SimpleAI/Art/Characters/Kachujin/Anim/Attack/Montage/AM_Kachujin_Fireball.AM_Kachujin_Fireball")
    (:OnCompleted
      (CallFunction|AttackEnd (Variables|Event_Attack|GetAttack_InAttackTarget) :!label _label))
    (:OnInterrupted
      (goto _label))
    (:OnNotifyBegin
      (switch name _notifyname
        (:Fire
          (Default|MagicSpell (Variables|Default|GetBPC_Attack) (Transformation|GetBoneTransform (Variables|Character|GetMesh) "RightHand" "RTS_World") (Variables|Event_Attack|GetAttack_InAttackTarget) (Utilities|Struct|MakeS_DamageInfo 2e+01 "NewEnumerator2" "NewEnumerator1")))))))

(fn ConstructionScript
  (|CallParentFunction))

(fn SetMovementSpeed
  (params (InSpeedType :type E_MovementSpeed%20Enum :default "NewEnumerator0"))
  (bind _output_get (Variables|/Script/Engine.CharacterMovementComponent|SetMaxWalkSpeed (Variables|Character|GetCharacterMovement) (Utilities|Select :Index InSpeedType :NewEnumerator0 0.0 :NewEnumerator1 1.5e+02 :NewEnumerator2 2.5e+02 :NewEnumerator3 4e+02)))
  (return _output_get))

(fn GetIdealRange
  (return 5e+02 7e+02))