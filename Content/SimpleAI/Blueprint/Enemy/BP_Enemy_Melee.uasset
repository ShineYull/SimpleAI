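; BP_Enemy_Melee is a sword-wielding AI enemy that overrides its parent's attack and adds montage-driven weapon handling and blocking.
; Montage notifies trigger a forward sphere trace that damages pawns, and spawn or destroy the hand-socketed sword on draw and sheathe.
; Attacks are uninterruptible through the damage component, whose OnBlocked dispatcher plays a block reaction.
; BlockingState keeps that reaction from ending the block early, and dispatchers announce equip, unequip and block completion.
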(event DispatcheronBlocked(BPC_Damage)
  (params (InCanBeParried :type Boolean))
  ;[0.15 0.15 0.15 0.5] 格挡招式
  (Variables|Default|SetBlockingState "NewEnumerator2")
  (Animation|Montage|PlayMontage (Variables|Character|GetMesh) "/Game/Characters/Mannequins/Anims/Sword/Block/AM_Sword_Blocking_React.AM_Sword_Blocking_React"
    (:OnCompleted
      _)
    (:OnInterrupted
      _))
  (CallFunction|EndBlock))

(event Custom|StartBlock
  ;[0.15 0.15 0.15 0.5] 格挡招式
  (Components|Movement|StopMovementImmediately (Variables|Character|GetCharacterMovement))
  (Variables|/Game/SimpleAI/Blueprint/Damage_Component/BPC_Damage.BPC_Damage_C|SetbIsBlocking (Variables|Default|GetBPC_Damage) true)
  (Variables|Default|SetBlockingState "NewEnumerator1")
  (Animation|Montage|PlayMontage (Variables|Character|GetMesh) "/Game/Characters/Mannequins/Anims/Sword/Block/AM_Sword_Blocking.AM_Sword_Blocking"
    (:OnCompleted
      (CallFunction|EndBlock :!label _label))
    (:OnInterrupted
      (if (Utilities|Enum|NotEqual(Enum) (Variables|Default|GetBlockingState) "NewEnumerator2")
        (goto _label)))))

(event Custom|EndBlock
  ;[0.15 0.15 0.15 0.5] 格挡招式
  (Variables|/Game/SimpleAI/Blueprint/Damage_Component/BPC_Damage.BPC_Damage_C|SetbIsBlocking (Variables|Default|GetBPC_Damage) false)
  (Variables|Default|SetBlockingState "NewEnumerator0")
  (Default|CallDispatcherBlockEnded))

(event EventUnequipWeapon
  ;[0.15 0.15 0.15 0.5] 收剑
  (bind _notifyname (Animation|Montage|PlayMontage (Variables|Character|GetMesh) "/Game/Characters/Mannequins/Anims/Sword/AM_Sheath_Sword.AM_Sheath_Sword")
    (:OnCompleted
      (Default|CallDispatcherUnequipWeaponCompleted))
    (:OnNotifyBegin
      (switch name _notifyname
        (:DropSword
          (Actor|DestroyActor (Variables|Default|GetWeaponActor))
          (Variables|Default|SetbIsWieldingWeapon false))))))

(event EventEquipWeapon
  ;[0.15 0.15 0.15 0.5] 拔剑
  (bind _notifyname (Animation|Montage|PlayMontage (Variables|Character|GetMesh) "/Game/Characters/Mannequins/Anims/Sword/AM_Draw_Sword.AM_Draw_Sword")
    (:OnCompleted
      (Default|CallDispatcherEquipWeaponCompleted))
    (:OnNotifyBegin
      (switch name _notifyname
        (:HoldSword
          (bind _returnvalue (Game|SpawnActorfromClass "/Game/SimpleAI/Blueprint/Weapon/BP_Weapon_Sword.BP_Weapon_Sword_C" (Transformation|GetActorTransform) "Undefined" "MultiplyWithRoot" 0 0))
          (Variables|Default|SetWeaponActor _returnvalue)
          (Transformation|AttachComponentToComponent (Variables|Default|GetWeaponActor) (Variables|Character|GetMesh) "Hand_R_Sword_Socket" "SnapToTarget" "SnapToTarget" "SnapToTarget" true)
          (Variables|Default|SetbIsWieldingWeapon true))))))

(event EventBeginPlay
  ;[0.15 0.15 0.15 0.5] 初始化
  (|CallParentFunction))

(event EventAttack
  (params (InAttackTarget :type Actor%20Object%20Reference))
  ;[0.15 0.15 0.15 0.5] 攻击
  (bind _output_get (Variables|Event_Attack|SetAttack_InAttackTarget InAttackTarget))
  (|CallParentFunction _output_get)
  (bind _notifyname (Animation|Montage|PlayMontage (Variables|Character|GetMesh) "/Game/Characters/Mannequins/Anims/Sword/AM_Sword_Slash.AM_Sword_Slash")
    (:then
      (Variables|/Game/SimpleAI/Blueprint/Damage_Component/BPC_Damage.BPC_Damage_C|SetbIsInterruptible (Variables|Default|GetBPC_Damage) false))
    (:OnCompleted
      (CallFunction|AttackEnd (Variables|Event_Attack|GetAttack_InAttackTarget) :!label _label)
      (Variables|/Game/SimpleAI/Blueprint/Damage_Component/BPC_Damage.BPC_Damage_C|SetbIsInterruptible (Variables|Default|GetBPC_Damage) true))
    (:OnInterrupted
      (goto _label))
    (:OnNotifyBegin
      (switch name _notifyname
        (:Slash
          (bind (_outhit _returnvalue) (Collision|SphereTraceForObjects (Transformation|GetActorLocation) (+ (Transformation|GetActorLocation) (* (Transformation|GetActorForwardVector) 2e+02)) 2e+01 (Utilities|Array|MakeArray "ObjectTypeQuery3") false 0 "ForDuration"))
          (if _returnvalue
            (Class|BPIDamagable|TakeDamage(Message) (.HitActor (Collision|BreakHitResult _outhit)) (Utilities|Struct|MakeS_DamageInfo 1.0 "NewEnumerator1") self)))))))

(fn ConstructionScript
  (|CallParentFunction))