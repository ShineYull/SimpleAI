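; Base projectile Blueprint for SimpleAI that flies at a set speed and gravity, optionally homing on a target actor.
; Construction configures the movement component and homing target; BeginPlay makes the box collision ignore the instigator (or owner) and aims velocity at any valid target.
; On hit, it broadcasts an impact dispatcher with the hit actor and result, spawns impact effect and sound, then destroys itself.
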(event Custom|RotateToTarget
  (Variables|/Script/Engine.MovementComponent|SetVelocity (Variables|Default|GetProjectileMovement) (* (Math|Vector|GetUnitDirection(Vector) (Transformation|GetActorLocation) (Transformation|GetActorLocation (Variables|Target|GetTargetActor))) (Variables|ProjectileSetting|GetSpeed))))

(event EventBeginPlay
  (Collision|IgnoreActorwhenMoving (Variables|Default|GetBoxCollision) (select (Utilities|IsValid (Game|GetInstigator)) (Game|GetInstigator) (Components|GetOwner)) true)
  (Variables|Target|GetTargetActor
    (:then
      (CallFunction|RotatetoTarget))
    (:else)))

(event OnComponentHit(BoxCollision)
  (params (HitComponent :type Primitive%20Component%20Object%20Reference) (OtherActor :type Actor%20Object%20Reference) (OtherComp :type Primitive%20Component%20Object%20Reference) (NormalImpulse :type Vector :default "0, 0, 0") (Hit :type Hit%20Result%20Structure%20%28by%20ref%29))
  (Variables|Collision_Event|SetOtherActor OtherActor)
  (Variables|CollisionEvent|SetHitResult Hit)
  (Default|CallDispatcherProjectileImpact (Variables|Collision_Event|GetOtherActor) (Variables|CollisionEvent|GetHitResult))
  (Effects|SpawnEmitteratLocation (Variables|CollisionEvent|GetImpactEffect) (.Location (Collision|BreakHitResult (Variables|CollisionEvent|GetHitResult))))
  (Audio|PlaySoundatLocation (Variables|CollisionEvent|GetImpactSound) (.Location (Collision|BreakHitResult (Variables|CollisionEvent|GetHitResult))) "0, 0, 0" 1.0 1.0 0.0 0 0 0 0)
  (Actor|DestroyActor))

(fn ConstructionScript
  (Utilities|FlowControl|Sequence
    (:then_0
      (Variables|/Script/Engine.ProjectileMovementComponent|SetInitialSpeed (Variables|Default|GetProjectileMovement) (Variables|ProjectileSetting|GetSpeed))
      (Variables|/Script/Engine.ProjectileMovementComponent|SetMaxSpeed (Variables|Default|GetProjectileMovement) (Variables|ProjectileSetting|GetSpeed))
      (Variables|/Script/Engine.ProjectileMovementComponent|SetProjectileGravityScale (Variables|Default|GetProjectileMovement) (Variables|ProjectileSetting|GetGravity)))
    (:then_1
      (Variables|Target|GetTargetActor
        (:then
          (Variables|/Script/Engine.ProjectileMovementComponent|SetbIsHomingProjectile (Variables|Default|GetProjectileMovement) (Variables|ProjectileSetting|GetbIsHoming))
          (Variables|/Script/Engine.ProjectileMovementComponent|SetHomingTargetComponent (Variables|Default|GetProjectileMovement) (Variables|/Script/Engine.Actor|GetRootComponent (Variables|Target|GetTargetActor))))
        (:else)))))