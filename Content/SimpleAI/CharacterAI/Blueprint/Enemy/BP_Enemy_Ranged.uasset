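; Ranged enemy AI character that fights with a rifle, built on a parent enemy Blueprint.
; On BeginPlay it spawns a rifle, attaches it to the hand socket and signals that equipping is complete.
; Attack plays the fire montage, whose notify has BPCAttack fire a damaging bullet trace from weapon to target; completion or interruption ends the attack.
; It also supplies movement speeds per speed type and ideal attack and defend ranges.
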(event EventBeginPlay
  ;[0.15 0.15 0.15 0.5] 初始化
  (|CallParentFunction)
  (CallFunction|EquipWeapon))

(event EventEquipWeapon
  ;[0.15 0.15 0.15 0.5] 装备武器
  (bind _returnvalue (Game|SpawnActorfromClass "/Game/SimpleAI/CharacterAI/Blueprint/Weapon/BP_Weapon_Rifle.BP_Weapon_Rifle_C" (Math|Transform|MakeTransform "0, 0, 0" "0, 0, 0" "1.000000,1.000000,1.000000") "Undefined" "MultiplyWithRoot" 0 0))
  (Variables|Default|SetWeaponActor _returnvalue)
  (Transformation|AttachComponentToComponent (Variables|Default|GetWeaponActor) (Variables|Character|GetMesh) "Hand_R_Rifle_Socket" "SnapToTarget" "SnapToTarget" "SnapToTarget" true)
  (Variables|Default|SetbIsWieldingWeapon true)
  (Default|CallDispatcherEquipWeaponCompleted))

(event EventAttack
  (params (InAttackTarget :type Actor%20Object%20Reference))
  ;[0.15 0.15 0.15 0.5] Pawn的攻击接口
  (bind _output_get (Variables|Event_Attack|SetAttack_InAttackTarget InAttackTarget))
  (|CallParentFunction _output_get)
  (bind _notifyname (Animation|Montage|PlayMontage (Variables|Character|GetMesh) "/Game/SimpleAI/CharacterAI/Art/Characters/Mannequins/Anims/Rifle/AM_Rifle_Fire.AM_Rifle_Fire")
    (:OnCompleted
      (CallFunction|AttackEnd (Variables|Event_Attack|GetAttack_InAttackTarget) :!label _label))
    (:OnInterrupted
      (goto _label))
    (:OnNotifyBegin
      (switch name _notifyname
        (:Fire
          (Default|FireBullet (Variables|Default|GetBPC_Attack) (Transformation|GetActorLocation (Variables|Default|GetWeaponActor)) (Transformation|GetActorLocation (Variables|Event_Attack|GetAttack_InAttackTarget)) (Utilities|Struct|MakeS_DamageInfo 15.0 "NewEnumerator2" "NewEnumerator0" false true)))))))

(fn ConstructionScript
  (|CallParentFunction))

(fn SetMovementSpeed
  (params (InSpeedType :type E_MovementSpeed%20Enum :default "NewEnumerator0"))
  (bind _output_get (Variables|/Script/Engine.CharacterMovementComponent|SetMaxWalkSpeed (Variables|Character|GetCharacterMovement) (Utilities|Select :Index InSpeedType :NewEnumerator0 0.0 :NewEnumerator1 2e+02 :NewEnumerator2 3e+02 :NewEnumerator3 5e+02)))
  (LocalVariables|SetLocal_NewSpeedValue _output_get)
  (return (LocalVariables|GetLocal_NewSpeedValue)))

(fn GetIdealRange
  (return 6e+02 6e+02))