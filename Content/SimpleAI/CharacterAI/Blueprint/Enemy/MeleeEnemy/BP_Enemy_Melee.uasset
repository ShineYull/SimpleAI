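; BP_Enemy_Melee is a sword-wielding AI enemy with ground smash, short-range, long-range jump and spinning attacks.
; Each attack event passes its montage, damage and target to the BPCAttack component.
; Equip and unequip montage notifies spawn and attach or destroy the sword, and montage completion fires dispatchers.
; It also supplies ideal attack and defend ranges, plus a helper predicting an actor's future location from horizontal velocity.
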(event Custom|ShortRangeAttack
  (params (InAttackTarget :type Actor%20Object%20Reference))
  ;[0.15 0.15 0.15 0.5] 攻击
  (Default|PrimaryMeleeAttack (Variables|Default|GetBPC_Attack) (Utilities|Struct|MakeS_AttackInfo InAttackTarget "/Game/SimpleAI/CharacterAI/Art/Characters/Mannequins/Anims/Sword/Attack/AM_Sword_Slash.AM_Sword_Slash" (Utilities|Struct|MakeS_DamageInfo 1e+01 "NewEnumerator1" "NewEnumerator0" false true true)) 2e+01 2e+02))

(event Custom|LongRangeAttack
  (params (InAttackTarget :type Actor%20Object%20Reference))
  ;[0.15 0.15 0.15 0.5] 攻击
  (Default|LongRangeMeleeAttack (Variables|Default|GetBPC_Attack) (Utilities|Struct|MakeS_AttackInfo InAttackTarget "/Game/SimpleAI/CharacterAI/Art/Characters/Mannequins/Anims/Sword/Attack/AM_Sword_Jump_Attack.AM_Sword_Jump_Attack" (Utilities|Struct|MakeS_DamageInfo 1e+01 "NewEnumerator1" "NewEnumerator0" false true true)) 2e+01 2e+02))

(event Custom|GroundSmashAttack
  (params (InAttackTarget :type Actor%20Object%20Reference))
  ;[0.15 0.15 0.15 0.5] 攻击
  (Default|GroundSmash (Variables|Default|GetBPC_Attack) (Utilities|Struct|MakeS_AttackInfo InAttackTarget "/Game/SimpleAI/CharacterAI/Art/Characters/Mannequins/Anims/Sword/Attack/AM_Sword_Ground_Smash.AM_Sword_Ground_Smash" (Utilities|Struct|MakeS_DamageInfo 25.0 "NewEnumerator3")) 3e+02))

(event Custom|SpinningAttack
  (params (InAttackTarget :type Actor%20Object%20Reference))
  ;[0.15 0.15 0.15 0.5] 攻击
  (Default|SpinningAttack (Variables|Default|GetBPC_Attack) (Utilities|Struct|MakeS_AttackInfo InAttackTarget "/Game/SimpleAI/CharacterAI/Art/Characters/Mannequins/Anims/Sword/Attack/AM_Sword_Spinning_Attack.AM_Sword_Spinning_Attack" (Utilities|Struct|MakeS_DamageInfo 1e+01 "NewEnumerator1" "NewEnumerator0" false true)) 2e+02))

(event EventUnequipWeapon
  ;[0.15 0.15 0.15 0.5] 收剑
  (bind _notifyname (Animation|Montage|PlayMontage (Variables|Character|GetMesh) "/Game/SimpleAI/CharacterAI/Art/Characters/Mannequins/Anims/Sword/DrawAndSheathSword/AM_Sheath_Sword.AM_Sheath_Sword")
    (:OnCompleted
      (Default|CallDispatcherUnequipWeaponCompleted))
    (:OnNotifyBegin
      (switch name _notifyname
        (:DropSword
          (Actor|DestroyActor (Variables|Default|GetWeaponActor))
          (Variables|Default|SetbIsWieldingWeapon false))))))

(event EventEquipWeapon
  ;[0.15 0.15 0.15 0.5] 拔剑
  (bind _notifyname (Animation|Montage|PlayMontage (Variables|Character|GetMesh) "/Game/SimpleAI/CharacterAI/Art/Characters/Mannequins/Anims/Sword/DrawAndSheathSword/AM_Draw_Sword.AM_Draw_Sword")
    (:OnCompleted
      (Default|CallDispatcherEquipWeaponCompleted))
    (:OnNotifyBegin
      (switch name _notifyname
        (:HoldSword
          (bind _returnvalue (Game|SpawnActorfromClass "/Game/SimpleAI/CharacterAI/Blueprint/Weapon/BP_Weapon_Sword.BP_Weapon_Sword_C" (Transformation|GetActorTransform) "Undefined" "MultiplyWithRoot" 0 0))
          (Variables|Default|SetWeaponActor _returnvalue)
          (Transformation|AttachComponentToComponent (Variables|Default|GetWeaponActor) (Variables|Character|GetMesh) "Hand_R_Sword_Socket" "SnapToTarget" "SnapToTarget" "SnapToTarget" true)
          (Variables|Default|SetbIsWieldingWeapon true))))))

(event EventBeginPlay
  ;[0.15 0.15 0.15 0.5] 初始化
  (|CallParentFunction))

(fn ConstructionScript
  (|CallParentFunction)
  (Variables|Event_SpinMesh|SetMeshRotationBeforeSpin (Variables|/Script/Engine.SceneComponent|GetRelativeRotation (Variables|Character|GetMesh))))

(fn GetIdealRange
  (return 2e+02 4e+02))

(fn CalculateFutureActorLocation
  (params (InActor :type Actor%20Object%20Reference) (InTime :type Float%20%28double-precision%29))
  (return (+ (Transformation|GetActorLocation InActor) (* (* (Transformation|GetVelocity InActor) "1.000000,1.000000,0.000000") InTime))))