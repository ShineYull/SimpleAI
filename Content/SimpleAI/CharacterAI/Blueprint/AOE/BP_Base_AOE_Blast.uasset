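; Base area-of-effect blast actor in the SimpleAI character AI, handling the visual and audio side of a blast when triggered.
; Trigger runs the parent logic, then spawns the blast particle emitter attached to the root and plays the blast sound at the actor's location.
; The actor destroys itself when the emitter finishes, or after a short delay if no effect is assigned.
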(event Custom|SpawnBlastEffect
  (Variables|Default|GetBlastEffect
    (:then
      (bind _returnvalue (Effects|SpawnEmitterAttached (Variables|Default|GetBlastEffect) (Variables|Default|GetDefaultSceneRoot) "None"))
      (Variables|Default|SetBlastEffectEmitter _returnvalue)
      (EventDispatchers|BindEventtoOnSystemFinished (Variables|Default|GetBlastEffectEmitter) (EventDispatchers|CreateEvent :!event BlastEffectEmitteronSystemFinished)))
    (:else
      (Utilities|FlowControl|Delay 1.0)
      (Actor|DestroyActor))))

(event Custom|PlayBlastSound
  (Variables|Default|GetBlastSound
    (:then
      (Audio|PlaySoundatLocation (Variables|Default|GetBlastSound) (Transformation|GetActorLocation) "0, 0, 0" 1.0 1.0 0.0 0 0 0 0))
    (:else)))

(event EventBeginPlay
  (|CallParentFunction) ; This node is disabled and will not be called.\nDrag off pins to build functionality.
)

(event Collision|EventActorBeginOverlap
  (params (OtherActor :type Actor%20Object%20Reference)))

(event EventTick
  (params (DeltaSeconds :type Float%20%28single-precision%29)))

(event EventTrigger
  (|CallParentFunction)
  (CallFunction|SpawnBlastEffect)
  (CallFunction|PlayBlastSound))

(fn ConstructionScript
  (|CallParentFunction))

(fn BlastEffectEmitteronSystemFinished
  (params (PSystem :type Particle%20System%20Component%20Object%20Reference))
  (Actor|DestroyActor))