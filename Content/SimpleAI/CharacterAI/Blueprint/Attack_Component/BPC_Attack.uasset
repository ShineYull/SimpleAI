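; Attack component for AI characters that implements melee, leap, spin, ground smash, bullet and magic spell attacks.
; Montage attacks message the owner on start and end, with notifies triggering sphere traces, spawned AOE actors or dark-energy projectiles.
; Bullets use line traces, and trace and AOE damage skip same-team actors.
; The leap launches toward the target's predicted position with a distance-scaled arc, stopping movement on landing.
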(event Custom|MagicSpell
  (params (InSpawnTransform :type Transform) (InTargetActor :type Actor%20Object%20Reference) (InDamageInfo :type S%20Damage%20Info%20Structure) (InAlt :type Boolean))
  ;[0.15 0.15 0.15 0.5] 蒙太奇通知：攻击通知
  ;;[0.15 0.15 0.15 0.5] 发射魔法咒语
  (Variables|MagicSpell_Event|SetSpawnTransform InSpawnTransform)
  (Variables|MagicSpellEvent|SetTargetActor InTargetActor)
  (Variables|MagicSpellEvent|SetDamageInfo InDamageInfo)
  (Variables|MagicSpellEvent|SetMagicSpell_InAlt InAlt)
  (bind _returnvalue (Game|SpawnActorfromClass (select (Variables|MagicSpellEvent|GetMagicSpell_InAlt) "/Game/SimpleAI/CharacterAI/Blueprint/Projectiles/BP_Projectile_DarkEnergy_Alt.BP_Projectile_DarkEnergy_Alt_C" "/Game/SimpleAI/CharacterAI/Blueprint/Projectiles/BP_Projectile_DarkEnergy.BP_Projectile_DarkEnergy_C") (Variables|MagicSpell_Event|GetSpawnTransform) "Undefined" "MultiplyWithRoot" (Components|GetOwner) 1e+03 0.0 (Variables|MagicSpellEvent|GetTargetActor) false 0))
  (Variables|MagicSpellEvent|SetMagicProjectile _returnvalue)
  (EventDispatchers|BindEventtoDispatcherProjectileImpact (Variables|MagicSpellEvent|GetMagicProjectile) (delegate Custom|OnProjectileHit))
  (Collision|IgnoreActorwhenMoving (Actor|GetComponentbyClass (Components|GetOwner) "/Script/Engine.CapsuleComponent") (Variables|MagicSpellEvent|GetMagicProjectile) true))

(event Custom|OnProjectileHit
  (params (InOtherActor :type Actor%20Object%20Reference) (InHitResult :type Hit%20Result%20Structure))
  ;[0.15 0.15 0.15 0.5] 蒙太奇通知：攻击通知
  ;;[0.15 0.15 0.15 0.5] 发射魔法咒语
  (Variables|MagicSpellEvent|SetHit_OtherActor InOtherActor)
  (Variables|MagicSpellEvent|SetHitResult InHitResult)
  (Class|BPIDamagable|TakeDamage(Message) (Variables|MagicSpellEvent|GetHit_OtherActor) (Variables|MagicSpellEvent|GetDamageInfo) (Components|GetOwner))
  (Class|AISenseDamage|ReportDamageEvent (Variables|MagicSpellEvent|GetHit_OtherActor) (Components|GetOwner) (Utilities|Struct|BreakS_DamageInfo (Variables|MagicSpellEvent|GetDamageInfo)) (Transformation|GetActorLocation (Components|GetOwner)) "0, 0, 0" "None")
  (Default|CallDispatcherAttackEnd))

(event Custom|AOEDamage
  (params (InDamageRadius :type Float%20%28double-precision%29) (InDamageInfo :type S%20Damage%20Info%20Structure))
  ;[0.15 0.15 0.15 0.5] 蒙太奇通知：攻击通知
  ;;[0.15 0.15 0.15 0.5] 范围伤害通知
  (Variables|EventAOEDamage|SetAOEDamage_InDamageRadius InDamageRadius)
  (Variables|EventAOEDamage|SetAOEDamage_InDamageInfo InDamageInfo)
  (bind _returnvalue (Game|SpawnActorfromClass "/Game/SimpleAI/CharacterAI/Blueprint/AOE/BP_Base_AOE.BP_Base_AOE_C" (Math|Transform|MakeTransform (Transformation|GetActorLocation (Components|GetOwner)) "0, 0, 0" "1.000000,1.000000,1.000000") "Undefined" "MultiplyWithRoot" 0 true false false (.AsPawn (Utilities|Casting|CastToPawn (Components|GetOwner)))))
  (Variables|EventAOEDamage|SetAOEDamage_BaseAOE _returnvalue)
  (Variables|/Game/SimpleAI/CharacterAI/Blueprint/AOE/BP_Base_AOE.BP_Base_AOE_C|SetSphereRadius (Variables|EventAOEDamage|GetAOEDamage_BaseAOE) (Variables|EventAOEDamage|GetAOEDamage_InDamageRadius))
  (EventDispatchers|AssignDispatcheronAOEOverlapActor (Variables|EventAOEDamage|GetAOEDamage_BaseAOE) (delegate Custom|AOEDamageActor))
  (Default|Trigger (Variables|EventAOEDamage|GetAOEDamage_BaseAOE)))

(event Custom|AOEDamageActor
  (params (InActor :type Actor%20Object%20Reference))
  ;[0.15 0.15 0.15 0.5] 蒙太奇通知：攻击通知
  ;;[0.15 0.15 0.15 0.5] 范围伤害通知
  (bind _outteamnumber (Class|BPIDamagable|GetTeamNumber(Message) InActor))
  (bind _outteamnumber_2 (Class|BPIDamagable|GetTeamNumber(Message) (Components|GetOwner)))
  (if (!= _outteamnumber_2 _outteamnumber)
    (Class|BPIDamagable|TakeDamage(Message) InActor (Variables|EventAOEDamage|GetAOEDamage_InDamageInfo) (Components|GetOwner))))

(event Custom|OnLand
  (params (Hit :type Hit%20Result%20Structure%20%28by%20ref%29))
  ;[0.15 0.15 0.15 0.5] 蒙太奇通知：攻击通知
  ;;[0.15 0.15 0.15 0.5] 跳到攻击目标处
  (EventDispatchers|UnbindEventfromLandedDelegate (.AsCharacter (Utilities|Casting|CastToCharacter (Components|GetOwner))) (delegate Custom|OnLand))
  (Components|Movement|StopMovementImmediately (Variables|/Script/Engine.Character|GetCharacterMovement (.AsCharacter (Utilities|Casting|CastToCharacter (Components|GetOwner))))))

(event Custom|FireBullet
  (params (InTraceStart :type Vector) (InTraceEnd :type Vector) (InDamageInfo :type S%20Damage%20Info%20Structure))
  ;[0.15 0.15 0.15 0.5] 蒙太奇通知：攻击通知
  ;;[0.15 0.15 0.15 0.5] 发射子弹
  (Variables|FireBullet_Event|SetTraceStart InTraceStart)
  (Variables|FireBulletEvent|SetTraceEnd InTraceEnd)
  (Variables|FireBulletEvent|SetFireBullet_DamageInfo InDamageInfo)
  (bind (_outhits _returnvalue) (Class|KismetSystemLibrary|LineTraceMultiforObjects (Variables|FireBullet_Event|GetTraceStart) (Variables|FireBulletEvent|GetTraceEnd) (Utilities|Array|MakeArray "ObjectTypeQuery3") false (Utilities|Array|MakeArray (Components|GetOwner)) "None" true))
  (Variables|FireBulletEvent|SetFireBullet_HitResult _outhits)
  (if _returnvalue
    (bind _outdamagedactor (CallFunction|DamageFirstNonTeamMeber (Variables|FireBulletEvent|GetFireBullet_HitResult) (Variables|FireBulletEvent|GetFireBullet_DamageInfo)))
    (Variables|FireBulletEvent|SetFireBullet_OutDamagedActor _outdamagedactor)
    (Class|AISenseDamage|ReportDamageEvent (Variables|FireBulletEvent|GetFireBullet_OutDamagedActor) (Components|GetOwner) (Utilities|Struct|BreakS_DamageInfo (Variables|FireBulletEvent|GetFireBullet_DamageInfo)) (Transformation|GetActorLocation (Components|GetOwner)) "0, 0, 0" "None")))

(event Custom|JumpToAttackTarget
  (params (InAttackTarget :type Actor%20Object%20Reference))
  ;[0.15 0.15 0.15 0.5] 蒙太奇通知：攻击通知
  ;;[0.15 0.15 0.15 0.5] 跳到攻击目标处
  (bind _output_get (Variables|Event_JumpToAttackTarget|SetJumpToAttackTarget_InAttackTarget InAttackTarget))
  (bind _outlocation (CallFunction|CalculateFutureActorLocation _output_get 1.0))
  (bind _outlaunchvelocity (Game|SuggestProjectileVelocityCustomArc (Transformation|GetActorLocation (Components|GetOwner)) (Math|Vector|MakeVector (.x _outlocation) (.y _outlocation) (.z _outlocation)) 0.0 (Math|Float|Lerp 0.5 0.92 (Math|Float|Clamp(Float) (Math|Float|NormalizetoRange (Transformation|GetDistanceTo (Variables|Event_JumpToAttackTarget|GetJumpToAttackTarget_InAttackTarget) (Components|GetOwner)) 4e+02 8e+02)))))
  (Character|LaunchCharacter (.AsCharacter (Utilities|Casting|CastToCharacter (Components|GetOwner))) _outlaunchvelocity true true)
  (EventDispatchers|AssignLandedDelegate (.AsCharacter (Utilities|Casting|CastToCharacter (Components|GetOwner))) (delegate Custom|OnLand)))

(event Custom|LongRangeMeleeAttack
  (params (InAttackInfo :type S%20Attack%20Info%20Structure) (InRadius :type Float%20%28double-precision%29) (InLenght :type Float%20%28double-precision%29))
  ;[0.15 0.15 0.15 0.5] 近战的长距离跳跃攻击
  (Variables|Event_LongRangeAttack|SetLongRangeAttack_InAttackInfo InAttackInfo)
  (Variables|EventLongRangeAttack|SetLongRangeAttack_InRadius InRadius)
  (Variables|EventLongRangeAttack|SetLongRangeAttack_InLenght InLenght)
  (bind _outmesh (CallFunction|AttackBase (.attacktarget (Variables|Event_LongRangeAttack|GetLongRangeAttack_InAttackInfo))))
  (bind _notifyname (Animation|Montage|PlayMontage _outmesh (.animmontage (Variables|Event_LongRangeAttack|GetLongRangeAttack_InAttackInfo)))
    (:then
      (Class|BPIDamagable|SetIsInterruptible(Message) (Components|GetOwner) false))
    (:OnCompleted
      (Class|BPIEnemyAI|AttackEnd(Message) (Components|GetOwner) (.attacktarget (Variables|Event_LongRangeAttack|GetLongRangeAttack_InAttackInfo)) :!label _label)
      (Class|BPIDamagable|SetIsInterruptible(Message) (Components|GetOwner) true))
    (:OnInterrupted
      (goto _label))
    (:OnNotifyBegin
      (switch name _notifyname
        (:Slash
          (CallFunction|SphereTraceDamage (.damageinfo (Variables|Event_LongRangeAttack|GetLongRangeAttack_InAttackInfo)) (Variables|EventLongRangeAttack|GetLongRangeAttack_InRadius) (Variables|EventLongRangeAttack|GetLongRangeAttack_InLenght)))
        (:Jump
          (CallFunction|JumptoAttackTarget (.attacktarget (Variables|Event_LongRangeAttack|GetLongRangeAttack_InAttackInfo))))
        (:AOESlash
          (CallFunction|AOEDamage 3e+02 (.damageinfo (Variables|Event_LongRangeAttack|GetLongRangeAttack_InAttackInfo))))))))

(event Custom|SphereTraceDamage
  (params (InDamageInfo :type S%20Damage%20Info%20Structure) (InRadius :type Float%20%28double-precision%29) (InLenght :type Float%20%28double-precision%29))
  ;[0.15 0.15 0.15 0.5] 蒙太奇通知：攻击通知
  ;;[0.15 0.15 0.15 0.5] 球形追踪检测
  (Variables|Event_SphereTraceDamage|SetSphereTraceDamage_InDamageInfo InDamageInfo)
  (Variables|EventSphereTraceDamage|SetSphereTraceDamage_InRadius InRadius)
  (Variables|EventSphereTraceDamage|SetSphereTraceDamage_InLenght InLenght)
  (bind (_outhits _returnvalue) (Collision|MultiSphereTraceForObjects (Transformation|GetActorLocation (Components|GetOwner)) (+ (Transformation|GetActorLocation (Components|GetOwner)) (* (Transformation|GetActorForwardVector (Components|GetOwner)) (Variables|EventSphereTraceDamage|GetSphereTraceDamage_InLenght))) (Variables|EventSphereTraceDamage|GetSphereTraceDamage_InRadius) (Utilities|Array|MakeArray "ObjectTypeQuery3") false 0 "None"))
  (if _returnvalue
    (CallFunction|DamageAllNonTeamMebers _outhits (Variables|Event_SphereTraceDamage|GetSphereTraceDamage_InDamageInfo))))

(event Custom|PrimaryMeleeAttack
  (params (InAttackInfo :type S%20Attack%20Info%20Structure) (InRadius :type Float%20%28double-precision%29) (InLenght :type Float%20%28double-precision%29))
  ;[0.15 0.15 0.15 0.5] 主要近战攻击
  (Variables|Event_PrimaryMeleeAttack|SetPrimaryMeleeAttack_InAttackInfo InAttackInfo)
  (Variables|EventPrimaryMeleeAttack|SetPrimaryMeleeAttack_InRadius InRadius)
  (Variables|EventPrimaryMeleeAttack|SetPrimaryMeleeAttack_InLenght InLenght)
  (bind _outmesh (CallFunction|AttackBase (.attacktarget (Variables|Event_PrimaryMeleeAttack|GetPrimaryMeleeAttack_InAttackInfo))))
  (bind _notifyname (Animation|Montage|PlayMontage _outmesh (.animmontage (Variables|Event_PrimaryMeleeAttack|GetPrimaryMeleeAttack_InAttackInfo)))
    (:OnCompleted
      (Class|BPIEnemyAI|AttackEnd(Message) (Components|GetOwner) (.attacktarget (Variables|Event_PrimaryMeleeAttack|GetPrimaryMeleeAttack_InAttackInfo)) :!label _label))
    (:OnInterrupted
      (goto _label))
    (:OnNotifyBegin
      (switch name _notifyname
        (:Slash
          (CallFunction|SphereTraceDamage (.damageinfo (Variables|Event_PrimaryMeleeAttack|GetPrimaryMeleeAttack_InAttackInfo)) (Variables|EventPrimaryMeleeAttack|GetPrimaryMeleeAttack_InRadius) (Variables|EventPrimaryMeleeAttack|GetPrimaryMeleeAttack_InLenght)))))))

(event Custom|BarrageAttack
  (params (InAttackInfo :type S%20Attack%20Info%20Structure))
  ;[0.15 0.15 0.15 0.5] 弹幕法术攻击
  (Variables|Event_BarrageAttack|SetBarrageAttack_InAttackInfo InAttackInfo)
  (bind _outmesh (CallFunction|AttackBase (.attacktarget (Variables|Event_BarrageAttack|GetBarrageAttack_InAttackInfo))))
  (bind _notifyname (Animation|Montage|PlayMontage _outmesh (.animmontage (Variables|Event_BarrageAttack|GetBarrageAttack_InAttackInfo)))
    (:OnCompleted
      (Class|BPIEnemyAI|AttackEnd(Message) (Components|GetOwner) (.attacktarget (Variables|Event_BarrageAttack|GetBarrageAttack_InAttackInfo)) :!label _label)
      (Class|BPIDamagable|SetIsInterruptible(Message) (Components|GetOwner) true))
    (:OnInterrupted
      (goto _label))
    (:OnNotifyBegin
      (switch name _notifyname
        (:Fire
          (CallFunction|MagicSpell (Math|Transform|MakeTransform (Transformation|GetSocketLocation (Variables|/Script/Engine.Character|GetMesh (.AsCharacter (Utilities|Casting|CastToCharacter (Components|GetOwner)))) "RightHand") (Math|Rotator|FindLookatRotation (Transformation|GetActorLocation (Components|GetOwner)) (+ (Transformation|GetActorLocation (.attacktarget (Variables|Event_BarrageAttack|GetBarrageAttack_InAttackInfo))) (Math|Vector|MakeVector 0.0 (Math|Random|RandomFloatinRange -3e+02 3e+02) 0.0))) "1.000000,1.000000,1.000000") 0 (Utilities|Struct|MakeS_DamageInfo 1e+01 "NewEnumerator2" "NewEnumerator1") true)
          (Class|BPIDamagable|SetIsInterruptible(Message) (Components|GetOwner) false))))))

(event Custom|BasicMagicSpell
  (params (InAttackInfo :type S%20Attack%20Info%20Structure))
  ;[0.15 0.15 0.15 0.5] 基础法术攻击
  (Variables|Event_BasicMagicSpell|SetBasicMagicSpell_InAttackInfo InAttackInfo)
  (bind _outmesh (CallFunction|AttackBase (.attacktarget (Variables|Event_BasicMagicSpell|GetBasicMagicSpell_InAttackInfo))))
  (bind _notifyname (Animation|Montage|PlayMontage _outmesh (.animmontage (Variables|Event_BasicMagicSpell|GetBasicMagicSpell_InAttackInfo)))
    (:OnCompleted
      (Class|BPIEnemyAI|AttackEnd(Message) (Components|GetOwner) (.attacktarget (Variables|Event_BasicMagicSpell|GetBasicMagicSpell_InAttackInfo)) :!label _label))
    (:OnInterrupted
      (goto _label))
    (:OnNotifyBegin
      (switch name _notifyname
        (:Fire
          (CallFunction|MagicSpell (Math|Transform|MakeTransform (Transformation|GetSocketLocation (Variables|/Script/Engine.Character|GetMesh (.AsCharacter (Utilities|Casting|CastToCharacter (Components|GetOwner)))) "RightHand") "0, 0, 0" "1.000000,1.000000,1.000000") (.attacktarget (Variables|Event_BasicMagicSpell|GetBasicMagicSpell_InAttackInfo)) (.damageinfo (Variables|Event_BasicMagicSpell|GetBasicMagicSpell_InAttackInfo)) false))))))

(event Custom|GroundSmash
  (params (InAttackInfo :type S%20Attack%20Info%20Structure) (InDamageRadius :type Float%20%28double-precision%29))
  ;[0.15 0.15 0.15 0.5] 地面重击
  (Variables|Event_GroundSmash|SetGroundSmash_InAttackInfo InAttackInfo)
  (Variables|EventGroundSmash|SetGroundSmash_InDamageRadius InDamageRadius)
  (bind _outmesh (CallFunction|AttackBase (.attacktarget (Variables|Event_GroundSmash|GetGroundSmash_InAttackInfo))))
  (bind _notifyname (Animation|Montage|PlayMontage _outmesh (.animmontage (Variables|Event_GroundSmash|GetGroundSmash_InAttackInfo)))
    (:then
      (Class|BPIDamagable|SetIsInterruptible(Message) (Components|GetOwner) false))
    (:OnCompleted
      (Class|BPIEnemyAI|AttackEnd(Message) (Components|GetOwner) (.attacktarget (Variables|Event_GroundSmash|GetGroundSmash_InAttackInfo)) :!label _label)
      (Class|BPIDamagable|SetIsInterruptible(Message) (Components|GetOwner) true))
    (:OnInterrupted
      (goto _label))
    (:OnNotifyBegin
      (switch name _notifyname
        (:Smash
          (CallFunction|AOEDamage (Variables|EventGroundSmash|GetGroundSmash_InDamageRadius) (.damageinfo (Variables|Event_GroundSmash|GetGroundSmash_InAttackInfo))))))))

(event Custom|SpinningAttack
  (params (InAttackInfo :type S%20Attack%20Info%20Structure) (InAOEDamageRadius :type Float%20%28double-precision%29))
  ;[0.15 0.15 0.15 0.5] 旋转攻击
  (Variables|Event_SpinningAttack|SetSpinningAttack_InAttackInfo InAttackInfo)
  (Variables|EventSpinningAttack|SetSpinningAttack_InAOEDamageRadius InAOEDamageRadius)
  (bind _outmesh (CallFunction|AttackBase (.attacktarget (Variables|Event_SpinningAttack|GetSpinningAttack_InAttackInfo))))
  (bind _notifyname (Animation|Montage|PlayMontage _outmesh (.animmontage (Variables|Event_SpinningAttack|GetSpinningAttack_InAttackInfo)))
    (:then
      (Class|BPIDamagable|SetIsInterruptible(Message) (Components|GetOwner) true))
    (:OnCompleted
      (Class|BPIEnemyAI|AttackEnd(Message) (Components|GetOwner) (.attacktarget (Variables|Event_SpinningAttack|GetSpinningAttack_InAttackInfo)) :!label _label)
      (Class|BPIDamagable|SetIsInterruptible(Message) (Components|GetOwner) true))
    (:OnInterrupted
      (goto _label))
    (:OnNotifyBegin
      (switch name _notifyname
        (:Slash
          (CallFunction|SphereTraceDamage (.damageinfo (Variables|Event_SpinningAttack|GetSpinningAttack_InAttackInfo)) 2e+01 2e+02))
        (:AOESlash
          (CallFunction|AOEDamage (Variables|EventSpinningAttack|GetSpinningAttack_InAOEDamageRadius) (.damageinfo (Variables|Event_SpinningAttack|GetSpinningAttack_InAttackInfo))))))))

(fn DamageAllNonTeamMebers
  (params (InHitResults :type Array%20of%20Hit%20Result%20Structures) (InDamageInfo :type S%20Damage%20Info%20Structure))
  (for _array_element InHitResults
    (LocalVariables|SetElement_HitResult _array_element)
    (LocalVariables|SetLocal_HitActor (.HitActor (Collision|BreakHitResult (LocalVariables|GetElement_HitResult))))
    (bind _outteamnumber (Class|BPIDamagable|GetTeamNumber(Message) (LocalVariables|GetLocal_HitActor)))
    (LocalVariables|SetLocal_HitActorTeamNumber _outteamnumber)
    (bind _outteamnumber_2 (Class|BPIDamagable|GetTeamNumber(Message) (Components|GetOwner)))
    (LocalVariables|SetLocal_OwnerTeamNumber _outteamnumber_2)
    (if (and (!= (LocalVariables|GetLocal_HitActorTeamNumber) (LocalVariables|GetLocal_OwnerTeamNumber)) (not (Utilities|Array|ContainsItem (LocalVariables|GetLocal_ActorsDamagedSoFar) (LocalVariables|GetLocal_HitActor))))
      (Class|BPIDamagable|TakeDamage(Message) (LocalVariables|GetLocal_HitActor) InDamageInfo (Components|GetOwner))
      (Utilities|Array|AddUnique (LocalVariables|GetLocal_ActorsDamagedSoFar) (LocalVariables|GetLocal_HitActor))))
  (return (LocalVariables|GetLocal_ActorsDamagedSoFar)))

(fn DamageFirstNonTeamMeber
  (params (InHitResults :type Array%20of%20Hit%20Result%20Structures) (InDamageInfo :type S%20Damage%20Info%20Structure))
  (Utilities|FlowControl|Sequence
    (:then_0
      (bind _array_element (Utilities|Array|ForEachLoopwithBreak InHitResults :!label _label)
        (:LoopBody
          (LocalVariables|SetElement_HitResult _array_element)
          (bind _outteamnumber (Class|BPIDamagable|GetTeamNumber(Message) (Components|GetOwner)))
          (LocalVariables|SetLocal_OwnerTeamNumber _outteamnumber)
          (LocalVariables|SetLocal_HitActor (.HitActor (Collision|BreakHitResult (LocalVariables|GetElement_HitResult))))
          (bind _outteamnumber_2 (Class|BPIDamagable|GetTeamNumber(Message) (LocalVariables|GetLocal_HitActor)))
          (LocalVariables|SetLocal_HitActorTeamNumber _outteamnumber_2)
          (if (!= (LocalVariables|GetLocal_OwnerTeamNumber) (LocalVariables|GetLocal_HitActorTeamNumber))
            (Class|BPIDamagable|TakeDamage(Message) (LocalVariables|GetLocal_HitActor) InDamageInfo (Components|GetOwner))
            (goto _label Break)))))
    (:then_1
      (return (LocalVariables|GetLocal_HitActor)))))

(fn AttackBase
  (params (InAttackTarget :type Actor%20Object%20Reference))
  (Class|BPIEnemyAI|Attack(Message) (Components|GetOwner) InAttackTarget)
  (bind _ascharacter (Utilities|Casting|CastToCharacter (Components|GetOwner)))
  (return (Variables|/Script/Engine.Character|GetMesh _ascharacter)))

(fn CalculateFutureActorLocation
  (params (InActor :type Actor%20Object%20Reference) (InTime :type Float%20%28double-precision%29))
  (return (+ (Transformation|GetActorLocation InActor) (* (* (Transformation|GetVelocity InActor) "1.000000,1.000000,0.000000") InTime))))